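; Wall actor that swaps from a pulsing glow material to a dissolve material and fades away when the player is near.
; Two dynamic material instances are created at BeginPlay; SwapMaterial and shared scalar parameters select between them.
; Tick interpolates dissolve by player distance, reversing out of range or when IsDirty, which also restores pulsing once solid.
; Dissolve amount also drives the collision box's extent and disables its collision past a threshold.
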(event `self.ReceiveBeginPlay`
  (bind _dynamic_mat_dissolve (`self.dynamic_mat_dissolve`))
  (bind _dynamic_mat_pulsate (`self.dynamic_mat_pulsate`))
  ;[1 1 1] sets material dynamically
  (bind _returnvalue (`KismetMaterialLibrary.CreateDynamicMaterialInstance` "/Game/GuidingLight/TestStuff/ShaderStuff/RealtimeMaterials/M_DissolveMesh.M_DissolveMesh"))
  (set `self.dynamic_mat_dissolve` _returnvalue)
  (`MaterialInstanceDynamic.SetScalarParameterValue` _dynamic_mat_dissolve "Boost" (`self.boost_multiplyer`))
  (`MaterialInstanceDynamic.SetScalarParameterValue` _dynamic_mat_dissolve "Width" (`self.dissolve_width`))
  (`MaterialInstanceDynamic.SetScalarParameterValue` _dynamic_mat_dissolve "Amount" 0.0)
  (`MaterialInstanceDynamic.SetTextureParameterValue` _dynamic_mat_dissolve "Normal Map" (`self.normal_map`))
  (`MaterialInstanceDynamic.SetTextureParameterValue` _dynamic_mat_dissolve "Base Material" (`self.base_material`))
  (bind _returnvalue_2 (`KismetMaterialLibrary.CreateDynamicMaterialInstance` "/Game/GuidingLight/TestStuff/ShaderStuff/M_PulsateGlow_Bassalt_inst.M_PulsateGlow_Bassalt_inst"))
  (bind _output_get (set `self.dynamic_mat_pulsate` _returnvalue_2))
  (`PrimitiveComponent.SetMaterial` (`self.the_wall`) 0 _output_get)
  (`MaterialInstanceDynamic.SetTextureParameterValue` _dynamic_mat_pulsate "Normal Map" (`self.normal_map`))
  (`MaterialInstanceDynamic.SetTextureParameterValue` _dynamic_mat_pulsate "Texture map" (`self.base_material`))
  (`MaterialInstanceDynamic.SetVectorParameterValue` _dynamic_mat_pulsate "glow color" (struct :`R` 0.583333 :`B` 0.070165 :`A` 1.0)))

(event `self.ReceiveTick`
  (params (DeltaSeconds :type "Float (single-precision)"))
  (bind _box (`self.Box`))
  (`|ExecutionSequence`
    (:`then_0`
      (bind _returnvalue (`KismetMaterialLibrary.GetScalarParameterValue` null "AreWeDissolving"))
      (if (== _returnvalue 1.0)
        ;[1 1 1] sets how much has disolved if the player gets within a certian range
        (if (`self.IsDirty`)
          ;;[1 1 1] bring back
          (bind _returnvalue_2 (`MaterialInstanceDynamic.K2_GetScalarParameterValue` (`self.dynamic_mat_dissolve`) "Amount" :!label _label))
          (bind _returnvalue_3 (`KismetMathLibrary.FInterpTo_Constant` _returnvalue_2 0.0 DeltaSeconds (`self.dissolve_speed`)))
          (`MaterialInstanceDynamic.SetScalarParameterValue` (`self.dynamic_mat_dissolve`) "Amount" _returnvalue_3)
          (`MaterialInstanceDynamic.SetScalarParameterValue` (`self.dynamic_mat_dissolve`) "Boost" _returnvalue_3)
          (if (and (`KismetMathLibrary.NearlyEqual_FloatFloat` _returnvalue_3) (`self.IsDirty`))
            (set `self.swapMaterial` false)
            (`KismetMaterialLibrary.SetScalarParameterValue` null "AreWePulsating" 1.0)
            (`KismetMaterialLibrary.SetScalarParameterValue` null "AreWeDissolving")
            (`PrimitiveComponent.SetMaterial` (`self.the_wall`) 0 (`self.dynamic_mat_pulsate`)))
          (elif (<= (`self.GetDistanceTo` (`GameplayStatics.GetPlayerCharacter` 0) self) (`self.radius_of_influence`))
            ;;[1 1 1] dissolve away
            (bind _returnvalue_4 (`MaterialInstanceDynamic.K2_GetScalarParameterValue` (`self.dynamic_mat_dissolve`) "Amount"))
            (bind _returnvalue_5 (`KismetMathLibrary.FInterpTo_Constant` _returnvalue_4 1.0 DeltaSeconds (`self.dissolve_speed`)))
            (`MaterialInstanceDynamic.SetScalarParameterValue` (`self.dynamic_mat_dissolve`) "Amount" _returnvalue_5)
            (`MaterialInstanceDynamic.SetScalarParameterValue` (`self.dynamic_mat_dissolve`) "Boost" (* (`KismetMathLibrary.Sin` (* _returnvalue_5 1.570796)) (`self.boost_multiplyer`)))
            (else
              (goto _label))))
        (elif (`self.swapMaterial`)
          (`PrimitiveComponent.SetMaterial` (`self.the_wall`) 0 (`self.dynamic_mat_dissolve`))
          (set `self.swapMaterial` false)
          (`KismetMaterialLibrary.SetScalarParameterValue` null "AreWePulsating")
          (`KismetMaterialLibrary.SetScalarParameterValue` null "AreWeDissolving" 1.0)
          (set `self.IsDirty` false))))
    (:`then_1`
      ;[1 1 1] disables collision when the objet is invisible
      (bind _returnvalue_6 (`MaterialInstanceDynamic.K2_GetScalarParameterValue` (`self.dynamic_mat_dissolve`) "Amount"))
      (if (>= _returnvalue_6 (`self.bounding_box_disabled_percentage`))
        (`PrimitiveComponent.SetCollisionEnabled` _box "NoCollision")
        (else
          (`PrimitiveComponent.SetCollisionEnabled` _box "QueryAndPhysics"))))
    (:`then_2`
      (bind _returnvalue_7 (`MaterialInstanceDynamic.K2_GetScalarParameterValue` (`self.dynamic_mat_dissolve`) "Amount"))
      (if (!= _returnvalue_7 0.0)
        (bind _returnvalue_8 (* _returnvalue_7 2.0))
        (`BoxComponent.SetBoxExtent` (`self.Box`) (`KismetMathLibrary.MakeVector` _returnvalue_8 _returnvalue_8 _returnvalue_8) true)))))

(fn `UserConstructionScript`)
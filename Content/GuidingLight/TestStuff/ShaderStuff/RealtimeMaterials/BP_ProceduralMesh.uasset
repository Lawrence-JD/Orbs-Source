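; Test procedural mesh actor that can be sliced along a plane, capping the cut with CutFaceMaterial.
; The construction script applies the chosen mesh, material and scale, then copies the static mesh into a ProceduralMesh with collision.
; SliceMesh binds the plane's overlap to an empty handler, then immediately slices that handler's OtherComp at the plane, keeping both halves.
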(event `SliceMesh`
  (params (Plane :type "PrimitiveComponent Object Reference"))
  ;[1 1 1] Pass in a plane and it will subdivide the given mesh along that plane and set the inside material to the CutFaceMaterial
  (add `PrimitiveComponent.OnComponentBeginOverlap` Plane (delegate `CustomEvent`))
  (bind _asprocedural_mesh_component (cast `ProceduralMeshComponent` (stale `CustomEvent` OtherComp)))
  (`KismetProceduralMeshLibrary.SliceProceduralMesh` _asprocedural_mesh_component (`SceneComponent.K2_GetComponentLocation` Plane) (`SceneComponent.GetUpVector` Plane) true "CreateNewSectionForCap" (`self.CutFaceMaterial`)))

(event `CustomEvent`
  (params (OverlappedComponent :type "PrimitiveComponent Object Reference") (OtherActor :type "Actor Object Reference") (OtherComp :type "PrimitiveComponent Object Reference") (OtherBodyIndex :type Integer) (bFromSweep :type Boolean) (SweepResult :type "HitResult Structure (by ref)"))
  ;[1 1 1] Pass in a plane and it will subdivide the given mesh along that plane and set the inside material to the CutFaceMaterial
)

(fn `UserConstructionScript`
  (bind _staticmeshcomponent (`self.StaticMeshComponent`))
  (`StaticMeshComponent.SetStaticMesh` _staticmeshcomponent (`self.StaticMesh`))
  (`PrimitiveComponent.SetMaterial` _staticmeshcomponent 0 (`self.Material`))
  (`SceneComponent.SetWorldScale3D` _staticmeshcomponent (`self.Scale`))
  (`KismetProceduralMeshLibrary.CopyProceduralMeshFromStaticMeshComponent` (`self.StaticMeshComponent`) 0 (`self.ProceduralMesh`) true))
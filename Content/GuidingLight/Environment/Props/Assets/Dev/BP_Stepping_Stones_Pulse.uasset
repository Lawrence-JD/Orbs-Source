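; Stepping stone prop whose emissive glow pulses repeatedly once PulseLight is called.
; The construction script shows mesh variant A or B based on CurrentSteppingStone.
; BeginPlay creates that mesh's dynamic emissive material, sets it dark and enables player input.
; Tick prints timing debug values and, while pulsable, wraps elapsed time over the pulse length to drive color, glow and rim from curves.
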(event `self.ReceiveBeginPlay`
  (switch `/Game/GuidingLight/Environment/Props/Assets/Dev/E_Stepping_Stones` (`self.CurrentSteppingStone`)
    (:`NewEnumerator0`
      (bind _returnvalue (`PrimitiveComponent.CreateDynamicMaterialInstance` (`self.Stepping_Stone_A`) 1 "/Game/GuidingLight/Environment/Props/Materials/M_EmissiveColors.M_EmissiveColors" "None"))
      (bind _output_get (set `self.EmmisiveColor` _returnvalue)))
    (:`NewEnumerator1`
      (bind _returnvalue_2 (`PrimitiveComponent.CreateDynamicMaterialInstance` (`self.Stepping_Stone_B`) 0 "/Game/GuidingLight/Environment/Props/Materials/M_EmissiveColors.M_EmissiveColors" "None"))
      (set `self.EmmisiveColor` _returnvalue_2)))
  (`|ExecutionSequence`
    (:`then_0`
      (`MaterialInstanceDynamic.SetVectorParameterValue` _output_get "Color" (struct :`A` 1.0))
      (`MaterialInstanceDynamic.SetVectorParameterValue` _output_get "GlowColor" (struct :`A` 1.0))
      (`MaterialInstanceDynamic.SetVectorParameterValue` _output_get "NormalIntensity\\" (struct :`R` 1.0 :`G` 1.0 :`B` 1.0 :`A` 1.0)))
    (:`then_1`
      (`MaterialInstanceDynamic.SetScalarParameterValue` _output_get "EncompassingGlow" 0.001)
      (`MaterialInstanceDynamic.SetScalarParameterValue` _output_get "Rim" 0.0)
      (`MaterialInstanceDynamic.SetScalarParameterValue` _output_get "TileRepeat" 1.0))
    (:`then_2`
      (`MaterialInstanceDynamic.SetTextureParameterValue` _output_get "NormalTexture" "/Game/GuidingLight/Environment/Props/Materials/Textures/T_P_Pots/Pot_Base_Normal.Pot_Base_Normal"))
    (:`then_3`
      (`self.EnableInput` (`GameplayStatics.GetPlayerController` 0)))))

(event `self.ReceiveTick`
  (params (DeltaSeconds :type "Float (single-precision)"))
  (bind _emmisivecolor (`self.EmmisiveColor`))
  (bind _returnvalue (/ (`self.Elapsed Time`) (`self.Lenght of Pulse`)))
  (`KismetSystemLibrary.PrintString` (`KismetStringLibrary.Conv_DoubleToString` (`self.Elapsed Time`)))
  (`KismetSystemLibrary.PrintString` (`KismetStringLibrary.Conv_DoubleToString` (`self.Lenght of Pulse`)) true true (struct :`R` 1.0 :`B` 0.089234 :`A` 1.0))
  (if (`self.isPulsable`)
    (bind _output_get (set `self.Elapsed Time` (+ DeltaSeconds (`self.Elapsed Time`))))
    (if (> (* (`self.AlphaBetweenPulse`) _output_get) (`self.Lenght of Pulse`))
      (set `self.Elapsed Time` (- (* (`self.AlphaBetweenPulse`) (`self.Elapsed Time`)) (`self.Lenght of Pulse`)))
      (else
        (`MaterialInstanceDynamic.SetVectorParameterValue` _emmisivecolor "GlowColor" (`CurveLinearColor.GetLinearColorValue` (`self.GlowColorCurve`) _returnvalue))
        (`MaterialInstanceDynamic.SetVectorParameterValue` _emmisivecolor "Color" (`CurveLinearColor.GetLinearColorValue` (`self.ColorCurve`) _returnvalue))
        (`MaterialInstanceDynamic.SetScalarParameterValue` _emmisivecolor "Rim" (`CurveFloat.GetFloatValue` (`self.RimCurve`) _returnvalue))))))

(fn `PulseLight`
  (set `self.isPulsable` true))

(fn `UserConstructionScript`
  (bind _stepping_stone_b (`self.Stepping_Stone_B`))
  (bind _stepping_stone_a (`self.Stepping_Stone_A`))
  (switch `/Game/GuidingLight/Environment/Props/Assets/Dev/E_Stepping_Stones` (`self.CurrentSteppingStone`)
    (:`NewEnumerator0`
      (`SceneComponent.SetVisibility` _stepping_stone_b false false)
      (`SceneComponent.SetHiddenInGame` _stepping_stone_b true false)
      (`SceneComponent.SetHiddenInGame` _stepping_stone_a false false)
      (`SceneComponent.SetVisibility` _stepping_stone_a true false))
    (:`NewEnumerator1`
      (`SceneComponent.SetVisibility` _stepping_stone_a false false)
      (`SceneComponent.SetHiddenInGame` _stepping_stone_a true false)
      (`SceneComponent.SetHiddenInGame` _stepping_stone_b false false)
      (`SceneComponent.SetVisibility` _stepping_stone_b true false))))
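; Shadow puzzle pedestal prop with six columns, each paired with a puzzle piece, configured entirely in the Construction Script.
; A shared ColumnDistance sets the relative Y offset of columns and pieces, and PuzzlePieceHeight sets the height of the pieces.
; Each stand-in mesh comes from its own PuzzlePiece array, indexed by that slot's Decision variable.
; The event graph holds no active runtime logic.
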(fn `UserConstructionScript`
  (bind _columndistance (`self.ColumnDistance`))
  (bind _columndistance_2 (`self.ColumnDistance`))
  (bind _puzzlepieceheight (`self.PuzzlePieceHeight`))
  ;[1 1 1] Setting Column Distance
  (`SceneComponent.K2_SetRelativeLocation` (`self.Column`) (`KismetMathLibrary.MakeVector` 0.0 _columndistance) false false)
  (`SceneComponent.K2_SetRelativeLocation` (`self.Column2`) (`KismetMathLibrary.MakeVector` 0.0 _columndistance) false false)
  (`SceneComponent.K2_SetRelativeLocation` (`self.Column3`) (`KismetMathLibrary.MakeVector` 0.0 _columndistance) false false)
  (`SceneComponent.K2_SetRelativeLocation` (`self.Column4`) (`KismetMathLibrary.MakeVector` 0.0 _columndistance) false false)
  (`SceneComponent.K2_SetRelativeLocation` (`self.Column5`) (`KismetMathLibrary.MakeVector` 0.0 _columndistance) false false)
  (`SceneComponent.K2_SetRelativeLocation` (`self.Column6`) (`KismetMathLibrary.MakeVector` 0.0 _columndistance) false false)
  ;[1 1 1] PuzzlePieceLocation
  (`SceneComponent.K2_SetRelativeLocation` (`self.Piece_1`) (`KismetMathLibrary.MakeVector` 0.0 _columndistance_2 _puzzlepieceheight) false false)
  (`SceneComponent.K2_SetRelativeLocation` (`self.Piece_2`) (`KismetMathLibrary.MakeVector` 0.0 _columndistance_2 _puzzlepieceheight) false false)
  (`SceneComponent.K2_SetRelativeLocation` (`self.Piece_3`) (`KismetMathLibrary.MakeVector` 0.0 _columndistance_2 _puzzlepieceheight) false false)
  (`SceneComponent.K2_SetRelativeLocation` (`self.Piece_4`) (`KismetMathLibrary.MakeVector` 0.0 _columndistance_2 _puzzlepieceheight) false false)
  (`SceneComponent.K2_SetRelativeLocation` (`self.Piece_5`) (`KismetMathLibrary.MakeVector` 0.0 _columndistance_2 _puzzlepieceheight) false false)
  (`SceneComponent.K2_SetRelativeLocation` (`self.Piece_6`) (`KismetMathLibrary.MakeVector` 0.0 _columndistance_2 _puzzlepieceheight) false false)
  (`StaticMeshComponent.SetStaticMesh` (`self.SM_P_puzzlePieces_standIn_A_1`) (`|GetArrayItem` (`self.PuzzlePiece_1`) (`self.Piece1_Decision`)))
  (`StaticMeshComponent.SetStaticMesh` (`self.SM_P_puzzlePieces_standIn_B_1`) (`|GetArrayItem` (`self.PuzzlePiece_2`) (`self.Piece2_Decision`)))
  (`StaticMeshComponent.SetStaticMesh` (`self.SM_P_puzzlePieces_standIn_C_1`) (`|GetArrayItem` (`self.PuzzlePiece_3`) (`self.Piece3_Decision`)))
  (`StaticMeshComponent.SetStaticMesh` (`self.SM_P_puzzlePieces_standIn_D_1`) (`|GetArrayItem` (`self.PuzzlePiece_4`) (`self.Piece4_Decision`)))
  (`StaticMeshComponent.SetStaticMesh` (`self.SM_P_puzzlePieces_standIn_E_1`) (`|GetArrayItem` (`self.PuzzlePiece_5`) (`self.Piece5_Decision`)))
  (`StaticMeshComponent.SetStaticMesh` (`self.SM_P_puzzlePieces_standIn_F_1`) (`|GetArrayItem` (`self.PuzzlePiece_6`) (`self.Piece6_Decision`))))
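; BP_Moving_Platform is a prop platform that moves its Cube along a spline.
; A timeline maps TrackDistance to spline length and sets the Cube's world location without sweeping.
; The MessagePasser event plays or reverses the timeline according to its State input.
; While MActivated is set, Tick drives the timeline in the direction chosen by MAtEnd, which flips on each finish to ping-pong the platform.
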(event `/Game/WhereDoTheseBelong/Button_Interface.Message_Passer`
  (params (State :type Boolean))
  ;[1 1 1] Message Passer Toggle (State Machine)
  (switch `int` (`KismetMathLibrary.Conv_BoolToInt` State)
    (:`0`
      (bind (_direction _trackdistance) (`Timeline|SplineTimeline` :!via `Reverse` :!label _label)
        (:`Update`
          (`SceneComponent.K2_SetWorldLocation` (`self.Cube`) (`SplineComponent.GetLocationAtDistanceAlongSpline` (`self.Spline`) (* _trackdistance (`SplineComponent.GetSplineLength` (`self.Spline`))) "World") false false))
        (:`Finished`
          (set `self.mAtEnd` (not (`self.mAtEnd`))))))
    (:`1`
      (goto _label))))

(event `self.ReceiveTick`
  (params (DeltaSeconds :type "Float (single-precision)"))
  (switch `int` (`KismetMathLibrary.Conv_BoolToInt` (`self.mActivated`))
    (:`1`
      (switch `int` (`KismetMathLibrary.Conv_BoolToInt` (`self.mAtEnd`))
        (:`0`
          (goto _label))
        (:`1`
          (goto _label :!via `Reverse`))))))

(fn `UserConstructionScript`)
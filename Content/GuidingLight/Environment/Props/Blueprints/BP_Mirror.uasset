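; Rotatable mirror prop whose pivot turns once repeated IncrementRotation calls fill a progress value that decays over time.
; Tick plays or reverses a timeline by that threshold, with a C++ RotateHelper computing the rotation.
; On finish it starts a cooldown and flips the yaw direction if progress stayed full.
; Physics mirrors instead lock post rotation and XY, and either type turns translucent under the "Ghosted" collision profile.
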(event `self.ReceiveBeginPlay`
  (bind _sm_p_mirror_post (`self.SM_P_Mirror_Post`))
  ;[1 1 1] Set Starting Rotation
  (set `self.StartingRotation` (`SceneComponent.K2_GetComponentRotation` (`self.MirrorPivot`)))
  (set `self.StartingLocation` (`SceneComponent.K2_GetComponentLocation` _sm_p_mirror_post))
  (set `self.StartingBaseRotation` (`SceneComponent.K2_GetComponentRotation` _sm_p_mirror_post)))

(event `Play`
  ;[1 1 1] Rotation Timeline
  (bind (_direction _newtrack_0) (`Timeline|Timeline_0` :!label _label)
    (:`Update`
      (bind _returnvalue (`ARotateHelper.RotatorCalculate` (`self.ARotateHelper`) (`self.StartingRotation`) (`self.RotateBy`) _newtrack_0)) ; C++ Helper Function to be used alongside timeline.
      (`SceneComponent.K2_SetWorldRotation` (`self.MirrorPivot`) _returnvalue false false))
    (:`Finished`
      (`|ExecutionSequence`
        (:`then_0`
          (goto _label :!via `Stop`))
        (:`then_1`
          (`self.Complete`)
          (set `self.bCanRotate` false)
          (set `self.Cooldown` 1.0))))))

(event `Increment Rotation`
  ;[1 1 1] Add to Progress Event
  (if (`self.bCanRotate`)
    (if (< (`self.RotationProgress`) 0.0)
      (set `self.RotationProgress` 0.3)
      (else
        (set `self.RotationProgress` (`KismetMathLibrary.FMin` (+ (`self.RotationProgress`) 0.3) 1.1))))))

(event `Play from Start`
  ;[1 1 1] Rotation Timeline
  (goto _label :!via `PlayFromStart`))

(event `Reverse`
  ;[1 1 1] Rotation Timeline
  (goto _label :!via `Reverse`))

(event `self.ReceiveTick`
  (params (DeltaSeconds :type "Float (single-precision)"))
  (bind _sm_p_mirror_post (`self.SM_P_Mirror_Post`))
  ;[1 1 1] Tick - Checks Threshold. If progress > 1 rotate, if < 1 reverse
  (if (`self.bCanRotate`)
    (`|ExecutionSequence` :!label _label_2
      (:`then_0`
        (if (`self.bPhysicsMirror`)
          (`SceneComponent.K2_SetWorldRotation` _sm_p_mirror_post (`self.StartingBaseRotation`) false true)
          (`SceneComponent.K2_SetWorldLocation` _sm_p_mirror_post (`KismetMathLibrary.MakeVector` (.x (`self.StartingLocation`)) (.y (`self.StartingLocation`)) (.z (`SceneComponent.K2_GetComponentLocation` _sm_p_mirror_post))) false true)
          (else
            (set `self.RotationProgress` (`KismetMathLibrary.FMax` (- (`self.RotationProgress`) (* DeltaSeconds 0.25))))
            (if (>= (`self.RotationProgress`) 1.0)
              (if (`self.bIsRotating`)
                (`self.Play`)
                (else
                  (`self.Play from Start`)
                  (set `self.bIsRotating` true)))
              (elif (`self.bIsRotating`)
                (`self.Reverse`))))))
      (:`then_1`
        (if (== (`PrimitiveComponent.GetCollisionProfileName` (`self.SM_P_Mirror_Post`)) "Ghosted")
          (`PrimitiveComponent.SetMaterial` (`self.SM_P_Mirror_Post`) 0 "/Game/GuidingLight/TestStuff/ShaderStuff/MaterialTemplates/M_TranslucentFadeExample.M_TranslucentFadeExample")
          (`PrimitiveComponent.SetMaterial` (`self.SM_P_Mirror_Main`) 0 "/Game/GuidingLight/TestStuff/ShaderStuff/MaterialTemplates/M_TranslucentFadeExample.M_TranslucentFadeExample")
          (`PrimitiveComponent.SetMaterial` (`self.SM_P_Mirror_Main`) 1 "/Game/GuidingLight/TestStuff/ShaderStuff/MaterialTemplates/M_TranslucentFadeExample.M_TranslucentFadeExample")
          (else
            (`PrimitiveComponent.SetMaterial` (`self.SM_P_Mirror_Post`) 0 "/Game/GuidingLight/Environment/Props/Assets/lambert1.lambert1")
            (`PrimitiveComponent.SetMaterial` (`self.SM_P_Mirror_Main`) 0 "/Game/GuidingLight/Environment/Props/Materials/Mirror_Mat.Mirror_Mat")
            (`PrimitiveComponent.SetMaterial` (`self.SM_P_Mirror_Main`) 1 "/Game/GuidingLight/Environment/Props/Materials/Mirror_Mat.Mirror_Mat")))))
    (else
      (bind _output_get (set `self.Cooldown` (- (`self.Cooldown`) DeltaSeconds)))
      (if (<= _output_get 0.0)
        (set `self.bCanRotate` true)
        (goto _label_2)))))

(event `Complete`
  ;[1 1 1] Reset On Completion of Timeline
  (set `self.bIsRotating` false)
  (set `self.StartingRotation` (`SceneComponent.K2_GetComponentRotation` (`self.MirrorPivot`)))
  (if (>= (`self.RotationProgress`) 1.0)
    (set `self.RotationProgress` 0.0)
    (set `self.RotateBy` (`KismetMathLibrary.MakeRotator` (.roll (`self.RotateBy`)) (.pitch (`self.RotateBy`)) (* (.yaw (`self.RotateBy`)) -1.0)))
    (else
      (set `self.RotationProgress` 0.0))))

(fn `UserConstructionScript`)
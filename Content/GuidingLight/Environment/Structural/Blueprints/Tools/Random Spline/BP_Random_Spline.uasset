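; Construction-script spline tool that scatters static meshes at a set spacing along a spline for environment dressing.
; Each spawned component randomly receives one of four meshes using an unseeded roll, so the mesh choice is not stream-controlled.
; Optional macros vary yaw and XY/Z scale within set ranges using seeded random streams.
; The scale macro's selector also rolls zero, which has no case, leaving some meshes unscaled.
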(fn `UserConstructionScript`
  (bind _spline (`self.Spline`))
  (bind _rot_random (`self.Rot Random`))
  (bind _spacing (`self.spacing`))
  (bind _returned_mesh (`self.returned mesh`))
  (bind _scale_random (`self.Scale Random`))
  (for _index (range (+ (`.ReturnValue` (`KismetMathLibrary.FMod` (- (`SplineComponent.GetDistanceAlongSplineAtSplinePoint` _spline (- (`SplineComponent.GetNumberOfSplinePoints` _spline) 1)) (`SplineComponent.GetDistanceAlongSplineAtSplinePoint` _spline 0)) _spacing)) 1))
    (bind _returnvalue (`AddComponent|NODE_AddStaticMeshComponent-0` :`bManualAttachment` true :`RelativeTransform` (`KismetMathLibrary.MakeTransform` (`SplineComponent.GetLocationAtDistanceAlongSpline` _spline (* (`KismetMathLibrary.Conv_IntToDouble` _index) _spacing) "World"))))
    (set `self.returned mesh` _returnvalue)
    (switch `int` (`KismetMathLibrary.RandomIntegerInRange` 1 4)
      (:`1`
        (`StaticMeshComponent.SetStaticMesh` _returned_mesh (`self.mesh 1`))
        ;[1 1 1] Randomness
        (if _scale_random
          (`self.random scale`
            (:`out`
              _)))
        (if _rot_random
          (`self.random rotation`)))
      (:`2`
        (`StaticMeshComponent.SetStaticMesh` _returned_mesh (`self.Mesh 2`))
        (if _scale_random
          (`self.random scale`
            (:`out`
              _)))
        (if _rot_random
          (`self.random rotation`)))
      (:`3`
        (`StaticMeshComponent.SetStaticMesh` _returned_mesh (`self.Mesh 3`))
        (if _scale_random
          (`self.random scale`
            (:`out`
              _)))
        (if _rot_random
          (`self.random rotation`)))
      (:`4`
        (`StaticMeshComponent.SetStaticMesh` _returned_mesh (`self.Mesh 4`))
        (if _scale_random
          (`self.random scale`
            (:`out`
              _)))
        (if _rot_random
          (`self.random rotation`))))))
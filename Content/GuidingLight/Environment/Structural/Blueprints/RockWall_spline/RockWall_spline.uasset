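; RockWall_spline is a structural environment Blueprint that builds a rock wall along an editable spline.
; The construction script adds a spline mesh for each segment, picking a rock mesh from an array through a seeded random stream.
; Each mesh attaches to the spline, bends to its points and tangents along a configurable forward axis, and uses query-only collision.
; An X rotation variable rolls the whole spline, and the event graph has no active logic.
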(fn `UserConstructionScript`
  (bind _spline (`self.Spline`))
  (bind _rock_wall_array (`self.rock wall array`))
  (for _index (range (+ (- (`SplineComponent.GetNumberOfSplinePoints` _spline) 2) 1))
    (bind _returnvalue (`AddComponent|NODE_AddSplineMeshComponent-0`))
    (bind _output_get (set `self.mesh` (`|GetArrayItem` _rock_wall_array (`KismetMathLibrary.RandomIntegerInRangeFromStream` 0 (- (`KismetArrayLibrary.Array_Length` _rock_wall_array) 1) (`self.stream seed`)))))
    (`StaticMeshComponent.SetStaticMesh` _returnvalue _output_get)
    (`SceneComponent.K2_SetRelativeRotation` (`self.Spline`) (`KismetMathLibrary.MakeRotator` (`self.X rotation`)) false false)
    (`SceneComponent.K2_AttachToComponent` _returnvalue _spline "None" "KeepRelative" "KeepRelative" "KeepRelative" true)
    (bind (_location _tangent) (`SplineComponent.GetLocationAndTangentAtSplinePoint` _spline _index "Local"))
    (bind (_location_2 _tangent_2) (`SplineComponent.GetLocationAndTangentAtSplinePoint` _spline (+ _index 1) "Local"))
    (`SplineMeshComponent.SetStartAndEnd` _returnvalue _location _tangent _location_2 _tangent_2 true)
    (`SplineMeshComponent.SetForwardAxis` _returnvalue (`self.forward axis`) true)
    (`PrimitiveComponent.SetCollisionEnabled` _returnvalue "QueryOnly")))
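; BP_CrumblingDoor_float is a door that breaks away when the player character enters its trigger volume.
; The overlap enables physics on the door mesh and fires two radial force impulses a short delay apart.
; With the second impulse the mesh switches to a red emissive material, then after a few seconds loses collision and is destroyed.
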(event `self.trigger volume.OnComponentBeginOverlap`
  (params (OverlappedComponent :type "PrimitiveComponent Object Reference") (OtherActor :type "Actor Object Reference") (OtherComp :type "PrimitiveComponent Object Reference") (OtherBodyIndex :type Integer) (bFromSweep :type Boolean) (SweepResult :type "HitResult Structure (by ref)"))
  (cast `GuidingLightCharacter` OtherActor)
  (`PrimitiveComponent.SetSimulatePhysics` (`self.P_SM_Crumbling_Door_OT_A_DM`) true)
  (`RadialForceComponent.FireImpulse` (`self.RadialForce`))
  (`KismetSystemLibrary.Delay` 0.4)
  (`RadialForceComponent.FireImpulse` (`self.RadialForce 2`))
  (`PrimitiveComponent.SetMaterial` (`self.P_SM_Crumbling_Door_OT_A_DM`) 0 "/Game/Material/M_RedEmissive.M_RedEmissive")
  (`KismetSystemLibrary.Delay` 4.0)
  (`PrimitiveComponent.SetCollisionEnabled` (`self.P_SM_Crumbling_Door_OT_A_DM`) "NoCollision")
  (`ActorComponent.K2_DestroyComponent` (`self.P_SM_Crumbling_Door_OT_A_DM`)))

(fn `UserConstructionScript`)
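; BP_NPC_R is a patrolling AI character that reacts to being hit by a RockPillar.
; When its PillarCollider overlaps a RockPillar, it launches itself upward with a random horizontal nudge, overriding only vertical velocity.
; It then sets the stunned flag on its blackboard, leaving any further stun behavior outside this Blueprint.
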(event `self.PillarCollider.OnComponentBeginOverlap`
  (params (OverlappedComponent :type "PrimitiveComponent Object Reference") (OtherActor :type "Actor Object Reference") (OtherComp :type "PrimitiveComponent Object Reference") (OtherBodyIndex :type Integer) (bFromSweep :type Boolean) (SweepResult :type "HitResult Structure (by ref)"))
  ;[1 1 1] If the pillar collides, launch the guy
  (cast `RockPillar` OtherActor)
  (`self.LaunchCharacter` self (`KismetMathLibrary.MakeVector` (`KismetMathLibrary.Conv_IntToDouble` (`KismetMathLibrary.RandomIntegerInRange` -200 200)) (`KismetMathLibrary.Conv_IntToDouble` (`KismetMathLibrary.RandomIntegerInRange` -200 200)) 1000.0) false true)
  (`BlackboardComponent.SetValueAsBool` (`AIBlueprintHelperLibrary.GetBlackboard` self) "b_isStunned" true))

(fn `UserConstructionScript`)
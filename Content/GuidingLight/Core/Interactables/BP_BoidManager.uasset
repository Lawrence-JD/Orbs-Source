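; Boid manager actor that steers its flock's targets, starting each boid on the manager at first tick.
; With SeekPlayer on, player overlap retargets the boids to the player; leaving arms a per-tick tether distance check.
; Past the tether, boids return to the manager or lose their target, per DefaultTargetSpawn.
; Logic for passing boid locations to materials through a canvas render target is disconnected.
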(event `self.InitBoidLocs`)

(event `self.UpdateBoidLocs`)

(event `self.ReceiveActorBeginOverlap`
  (params (OtherActor :type "Actor Object Reference"))
  (if (`self.SeekPlayer`)
    (if (== (`GameplayStatics.GetObjectClass` OtherActor) "/Game/GuidingLight/Core/Character/Crystal/ThirdPersonCharacter.ThirdPersonCharacter_C")
      (for _array_element (`self.Boids`)
        (set `Boid.Target` (`GameplayStatics.GetPlayerCharacter` 0) _array_element)))))

(event `self.ReceiveActorEndOverlap`
  (params (OtherActor :type "Actor Object Reference"))
  (if (`self.SeekPlayer`)
    (if (== (`GameplayStatics.GetObjectClass` OtherActor) "/Game/GuidingLight/Core/Character/Crystal/ThirdPersonCharacter.ThirdPersonCharacter_C")
      (set `self.CheckDist` true))))

(event `self.ReceiveTick`
  (params (DeltaSeconds :type "Float (single-precision)"))
  (`|ExecutionSequence`
    (:`then_0`
      (if (`self.CheckDist`)
        (if (>= (`KismetMathLibrary.VSize` (- (`self.K2_GetActorLocation` (`GameplayStatics.GetPlayerCharacter` 0)) (`self.K2_GetActorLocation`))) (`self.TetherDist`))
          (set `self.CheckDist` false)
          (if (`self.DefaultTargetSpawn`)
            (for _array_element (`self.Boids`)
              (set `Boid.Target` self _array_element))
            (else
              (for _array_element_2 (`self.Boids`)
                (set `Boid.Target` null _array_element_2)))))))
    (:`then_1`
      (`/Engine/EditorBlueprintResources/StandardMacros.DoOnce` false
        (:`Completed`
          (if (`self.DefaultTargetSpawn`)
            (for _array_element_3 (`self.Boids`)
              (set `Boid.Target` self _array_element_3))))))))

(fn `UserConstructionScript`)
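; Turntable interactable that turns its static mesh one 60-degree step each time RotateEvent fires.
; RotateEvent stores the starting rotation and plays a timeline, whose value feeds the C++ ARotateHelper to set the mesh's world rotation every update.
; IsRotating is true during the turn.
; On finish it clears and RotationIndex advances, wrapping from 5 to 0 to track six positions.
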(event `RotateEvent`
  (bind _rotationindex (`self.RotationIndex`))
  ;[1 1 1] Set Starting Variables and Begin Timeline
  (set `self.StartingRotation` (`SceneComponent.K2_GetComponentRotation` (`self.StaticMeshComponent`)))
  (set `self.bIsRotating` true)
  (bind (_direction _newtrack_0) (`Timeline|Timeline_0` :!via `PlayFromStart`)
    (:`Update`
      ;[1 1 1] Rotating The Turntable Every Frame During Timeline
      (bind _returnvalue (`ARotateHelper.RotatorCalculate` (`self.ARotateHelper`) (`self.StartingRotation`) (struct :`Yaw` 60.0) _newtrack_0)) ; C++ Helper Function to be used alongside timeline.
      (`SceneComponent.K2_SetWorldRotation` (`self.StaticMeshComponent`) _returnvalue false false))
    (:`Finished`
      ;[1 1 1] Upon the timeline finishing, increment the "Rotation Index" variable
      (set `self.bIsRotating` false)
      (if (<= _rotationindex 4)
        (set `self.RotationIndex` (+ _rotationindex 1)) ; <= 4, Add 1
        (else
          (set `self.RotationIndex` 0) ; after 5, reset to 0
        )))))

(fn `UserConstructionScript`)
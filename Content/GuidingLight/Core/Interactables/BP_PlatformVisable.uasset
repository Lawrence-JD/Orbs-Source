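; BP_PlatformVisable is a platform actor that bobs up and down while slowly spinning in place.
; On BeginPlay it plays the CustomSines timeline with a random time up to RangeCapNewTime, which can vary the phase between instances.
; Each update sets the Trans component's relative height from the sine track scaled by BouncyMultiplier and adds a small fixed yaw step, so spin speed depends on frame rate.
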(event `self.ReceiveBeginPlay`
  (bind (_direction _normal_sine) (`Timeline|Custom Sines` :`NewTime` (`KismetMathLibrary.RandomFloatInRange` 0.0 (`self.RangeCap New Time`)))
    (:`Update`
      (`SceneComponent.K2_SetRelativeTransform` (`self.Trans`) (`KismetMathLibrary.MakeTransform` (`KismetMathLibrary.MakeVector` 0.0 0.0 (* (* _normal_sine 10.0) (`self.BouncyMultiplier`))) (`KismetMathLibrary.MakeRotator` 0.0 0.0 (+ (`self.CurrentRotation`) 0.006))) false false)
      (set `self.CurrentRotation` (.yaw (`SceneComponent.RelativeRotation` (`self.Trans`)))))))

(fn `UserConstructionScript`)
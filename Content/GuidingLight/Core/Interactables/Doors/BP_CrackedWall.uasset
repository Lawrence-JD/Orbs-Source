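; BP_CrackedWall is a door-style cracked wall that adds screen shake and controller rumble while it moves.
; Every Tick it switches on its door State, and while opening or closing with the player within MaxDistance it plays a world camera shake and starts dynamic force feedback.
; Rumble intensity is set to fall off linearly with player distance, and the Open and Closed states stop it.
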(event `self.ReceiveTick`
  (params (DeltaSeconds :type "Float (single-precision)"))
  (bind _returnvalue (`self.K2_GetActorLocation`))
  (bind _maxdistance (`self.MaxDistance`))
  (bind _returnvalue_2 (`KismetMathLibrary.Abs` (`KismetMathLibrary.Vector_Distance` (`self.K2_GetActorLocation` (`GameplayStatics.GetPlayerCharacter` 0)) _returnvalue)))
  (switch `EDoorState` (`self.State`)
    (:`Closed`
      (goto _label :!via `Stop`))
    (:`Closing`
      _)
    (:`Opening`
      _)
    (:`Open`
      (goto _label :!via `Stop`)))
  (if (<= _returnvalue_2 _maxdistance)
    (`GameplayStatics.PlayWorldCameraShake` "/Game/GuidingLight/Effects/Environment/Haptic/SHAKEspeare.SHAKEspeare_C" _returnvalue (`self.MaxDistance`))
    (`PlayerController.PlayDynamicForceFeedback` (`GameplayStatics.GetPlayerController` 0) (* (- 1.0 (/ _returnvalue_2 _maxdistance)) (`self.MaxIntensity`)) 2.0 true true true true :!label _label)))

(fn `UserConstructionScript`)
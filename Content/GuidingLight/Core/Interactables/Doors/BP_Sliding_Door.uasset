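; BP_Sliding_Door is an interactable door that slides open and shut along a spline.
; MessagePasser plays or reverses the DoorSlide timeline according to the incoming State, while ToggleDoor flips an internal Toggle to do the same.
; The timeline's track value scales the spline length to set the door's world location along the path, without sweeping.
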(event `/Game/WhereDoTheseBelong/Button_Interface.Message_Passer`
  (params (State :type Boolean))
  (switch `int` (`KismetMathLibrary.Conv_BoolToInt` State)
    (:`0`
      (bind (_direction _trackdistance) (`Timeline|DoorSlide` :!via `Reverse` :!label _label)
        (:`Update`
          (`SceneComponent.K2_SetWorldLocation` (`self.Door`) (`SplineComponent.GetLocationAtDistanceAlongSpline` (`self.Spline`) (* _trackdistance (`SplineComponent.GetSplineLength` (`self.Spline`))) "World") false false))))
    (:`1`
      (goto _label))))

(event `ToggleDoor`
  (bind _output_get (set `self.Toggle` (not (`self.Toggle`))))
  (switch `int` (`KismetMathLibrary.Conv_BoolToInt` _output_get)
    (:`0`
      (goto _label :!via `Reverse`))
    (:`1`
      (goto _label))))

(fn `UserConstructionScript`)
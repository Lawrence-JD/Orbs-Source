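; An amplifier lamp post interactable that emits a laser beam from its arrow component.
; Its C++ Emitter is initialized with colored laser materials, mirror and receiver physical materials, the beam Blueprint, a trace channel and itself as the amplifier.
; Tick re-casts the ray through a short Delay, passing origin, direction, distance and a reflection limit, while the ray logic lives in C++.
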(event `self.ReceiveBeginPlay`
  ;[1 1 1] Initialization of values in CPP
  (`LaserEmitterComponent.InitAll` (`self.Emitter`) "/Game/GuidingLight/Environment/Props/Materials/M_Laser_Red.M_Laser_Red" "/Game/GuidingLight/Environment/Props/Materials/M_Laser_Yellow.M_Laser_Yellow" "/Game/GuidingLight/Environment/Props/Materials/M_Laser_Blue.M_Laser_Blue" "/Game/GuidingLight/Environment/Props/Materials/PM_MirrorPhys.PM_MirrorPhys" "/Game/GuidingLight/Environment/Props/Materials/PM_RecieverPhys.PM_RecieverPhys" self "/Game/GuidingLight/Core/Interactables/LaserBeam/BP_LaserBeam.BP_LaserBeam" "ECC_GameTraceChannel3")
  (`self.CastRayEv`))

(event `self.ReceiveTick`
  (params (DeltaSeconds :type "Float (single-precision)"))
  (`KismetSystemLibrary.Delay` 0.05)
  (`self.CastRayEv`))

(event `CastRayEv`
  (bind _arrow (`self.Arrow`))
  ;[1 1 1] Attaches needed values to call the cast ray function, further doc in CPP
  (`LaserEmitterComponent.CastRay` (`self.Emitter`) (`SceneComponent.K2_GetComponentLocation` _arrow) (`SceneComponent.GetForwardVector` _arrow) (`self.fDist`) (`self.imaxReflects`)))

(fn `UserConstructionScript`)
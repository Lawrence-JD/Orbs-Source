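; BP_TurnWheel is an interactable wheel that the player operates by holding the Hell input action.
; Collision overlap opens and closes a gate, so a press only takes effect while the ThirdPersonCharacter is in range.
; Pressing yaws the character toward the wheel, sets its RotatingWheel flag, disables movement and marks the wheel Active.
; Release restores walking and clears both flags; the wheel's own rotation is absent from these graphs.
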(event `self.ReceiveBeginPlay`
  (`self.EnableInput` (`GameplayStatics.GetPlayerController` 0)))

(event `InputAction|Hell` :consume false
  (params (Key :type "Key Structure"))
  (:`Pressed`
    (`/Engine/EditorBlueprintResources/StandardMacros.Gate` true :!label _label
      (:`Exit`
        (bind (_returnvalue_roll _returnvalue_pitch) (`KismetMathLibrary.BreakRotator` (`self.K2_GetActorRotation` (stale `self.Collision.OnComponentBeginOverlap` _asthird_person_character))))
        (bind (_returnvalue_x _returnvalue_y _returnvalue_z) (`KismetMathLibrary.BreakVector` (`self.K2_GetActorLocation` (stale `self.Collision.OnComponentBeginOverlap` _asthird_person_character))))
        (bind (_returnvalue_roll_2 _returnvalue_pitch_2 _returnvalue_yaw) (`KismetMathLibrary.BreakRotator` (`KismetMathLibrary.FindLookAtRotation` (`KismetMathLibrary.MakeVector` _returnvalue_x _returnvalue_y _returnvalue_z) (`self.K2_GetActorLocation`))))
        ;[1 1 1] Lock Player into Rotating Animation
        (`self.K2_SetActorRotation` (stale `self.Collision.OnComponentBeginOverlap` _asthird_person_character) (`KismetMathLibrary.MakeRotator` _returnvalue_roll _returnvalue_pitch _returnvalue_yaw) false)
        (set `GuidingLightCharacter.bRotatingWheel` true (stale `self.Collision.OnComponentBeginOverlap` _asthird_person_character))
        (`CharacterMovementComponent.SetMovementMode` (`Character.CharacterMovement` (stale `self.Collision.OnComponentBeginOverlap` _asthird_person_character)) "MOVE_None" 0)
        (set `self.Active` true))))
  (:`Released`
    (set `self.Active` false)
    ;[1 1 1] Reset Player Animation to Base
    (bind _asthird_person_character (cast `/Game/GuidingLight/Core/Character/Crystal/ThirdPersonCharacter` (`GameplayStatics.GetPlayerCharacter` 0)))
    (set `GuidingLightCharacter.bRotatingWheel` false _asthird_person_character)
    (`CharacterMovementComponent.SetMovementMode` (`Character.CharacterMovement` _asthird_person_character) "MOVE_Walking" 0)))

(event `self.Collision.OnComponentBeginOverlap`
  (params (OverlappedComponent :type "PrimitiveComponent Object Reference") (OtherActor :type "Actor Object Reference") (OtherComp :type "PrimitiveComponent Object Reference") (OtherBodyIndex :type Integer) (bFromSweep :type Boolean) (SweepResult :type "HitResult Structure (by ref)"))
  (bind _asthird_person_character (cast `/Game/GuidingLight/Core/Character/Crystal/ThirdPersonCharacter` OtherActor))
  (goto _label :!via `Open`))

(event `self.Collision.OnComponentEndOverlap`
  (params (OverlappedComponent :type "PrimitiveComponent Object Reference") (OtherActor :type "Actor Object Reference") (OtherComp :type "PrimitiveComponent Object Reference") (OtherBodyIndex :type Integer))
  (cast `/Game/GuidingLight/Core/Character/Crystal/ThirdPersonCharacter` OtherActor)
  (set `self.Active` false)
  (goto _label :!via `Close`))

(fn `UserConstructionScript`)
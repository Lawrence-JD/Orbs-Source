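; BP_Mirror is a rotatable mirror for the laser beam interactables, turned by repeatedly incrementing a progress value.
; IncrementRotation builds progress that Tick drains, playing the rotation timeline at full progress and reversing it when progress drops.
; A C++ helper, ARotateHelper, converts timeline values into the mesh's world rotation.
; On finish, it stores the new start rotation, resets progress and flips yaw direction if progress was still full.
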(event `Play`
  ;[1 1 1] Rotation Timeline
  (bind (_direction _newtrack_0) (`Timeline|Timeline_0` :!label _label)
    (:`Update`
      (bind _returnvalue (`ARotateHelper.RotatorCalculate` (`self.ARotateHelper`) (`self.StartingRotation`) (`self.RotateBy`) _newtrack_0)) ; C++ Helper Function to be used alongside timeline.
      (`SceneComponent.K2_SetWorldRotation` (`self.Mesh`) _returnvalue false false))
    (:`Finished`
      (`|ExecutionSequence`
        (:`then_0`
          (goto _label :!via `Stop`))
        (:`then_1`
          (`self.Complete`))))))

(event `self.ReceiveBeginPlay`
  ;[1 1 1] Set Starting Rotation
  (set `self.StartingRotation` (`SceneComponent.K2_GetComponentRotation` (`self.Mesh`))))

(event `Increment Rotation`
  ;[1 1 1] Add to Progress Event
  (if (< (`self.RotationProgress`) 0.0)
    (set `self.RotationProgress` 0.3)
    (else
      (set `self.RotationProgress` (`KismetMathLibrary.FMin` (+ (`self.RotationProgress`) 0.3) 1.1)))))

(event `Play from Start`
  ;[1 1 1] Rotation Timeline
  (goto _label :!via `PlayFromStart`))

(event `Reverse`
  ;[1 1 1] Rotation Timeline
  (goto _label :!via `Reverse`))

(event `Complete`
  ;[1 1 1] Reset On Completion of Timeline
  (set `self.bIsRotating` false)
  (set `self.StartingRotation` (`SceneComponent.K2_GetComponentRotation` (`self.Mesh`)))
  (if (>= (`self.RotationProgress`) 1.0)
    (set `self.RotationProgress` 0.0)
    (set `self.RotateBy` (`KismetMathLibrary.MakeRotator` (.roll (`self.RotateBy`)) (.pitch (`self.RotateBy`)) (* (.yaw (`self.RotateBy`)) -1.0)))
    (else
      (set `self.RotationProgress` 0.0))))

(event `self.ReceiveTick`
  (params (DeltaSeconds :type "Float (single-precision)"))
  ;[1 1 1] Tick - Checks Threshold. If progress > 1 rotate, if < 1 reverse
  (set `self.RotationProgress` (`KismetMathLibrary.FMax` (- (`self.RotationProgress`) (* DeltaSeconds 0.25))))
  (if (>= (`self.RotationProgress`) 1.0)
    (if (`self.bIsRotating`)
      (`self.Play`)
      (else
        (`self.Play from Start`)
        (set `self.bIsRotating` true)))
    (elif (`self.bIsRotating`)
      (`self.Reverse`))))

(fn `UserConstructionScript`)
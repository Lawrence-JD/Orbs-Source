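; Laser emitter interactable that casts a reflecting beam, set up with red, yellow and blue laser materials.
; BeginPlay hands EmitterClass the beam Blueprint, trace channel and physical materials for mirrors and receivers, then calls Activate with false.
; Tick, throttled by a short Delay, has EmitterClass cast a ray from the Arrow component, limited by distance and maximum reflection count.
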(event `self.ReceiveBeginPlay`
  (`LaserEmitterComponent.InitAll` (`self.EmitterClass`) "/Game/GuidingLight/Environment/Props/Materials/M_Laser_Red.M_Laser_Red" "/Game/GuidingLight/Environment/Props/Materials/M_Laser_Yellow.M_Laser_Yellow" "/Game/GuidingLight/Environment/Props/Materials/M_Laser_Blue.M_Laser_Blue" "/Game/GuidingLight/Environment/Props/Materials/PM_MirrorPhys.PM_MirrorPhys" "/Game/GuidingLight/Environment/Props/Materials/PM_RecieverPhys.PM_RecieverPhys" null "/Game/GuidingLight/Core/Interactables/LaserBeam/BP_LaserBeam.BP_LaserBeam" "ECC_WorldStatic")
  (`ActorComponent.Activate` (`self.EmitterClass`) false))

(event `self.ReceiveTick`
  (params (DeltaSeconds :type "Float (single-precision)"))
  (bind _arrow (`self.Arrow`))
  (`KismetSystemLibrary.Delay` 0.01)
  (`LaserEmitterComponent.CastRay` (`self.EmitterClass`) (`SceneComponent.K2_GetComponentLocation` _arrow) (`SceneComponent.GetForwardVector` _arrow) (`self.fDist`) (`self.imaxReflects`)))

(fn `UserConstructionScript`)
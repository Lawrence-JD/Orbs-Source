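; Checkpoint actor that saves the player's respawn location and red, blue and yellow orb inventory to the "CheckPoint" save slot.
; Overlapping CheckPoint1 creates the save, with controller rumble, or updates it when this checkpoint is not already current, spawning a particle effect.
; CheckPoint2 jumps into the same update path without checking that a save exists, relying on the player reference CheckPoint1 caches.
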(event `self.ReceiveTick`
  (params (DeltaSeconds :type "Float (single-precision)")))

(event `self.CheckPoint1.OnComponentBeginOverlap`
  (params (OverlappedComponent :type "PrimitiveComponent Object Reference") (OtherActor :type "Actor Object Reference") (OtherComp :type "PrimitiveComponent Object Reference") (OtherBodyIndex :type Integer) (bFromSweep :type Boolean) (SweepResult :type "HitResult Structure (by ref)"))
  (bind _crystal (`self.Crystal`))
  (bind _playersettings (`self.PlayerSettings`))
  (bind _playersettings_2 (`self.PlayerSettings`))
  (bind _playersettings_3 (`self.PlayerSettings`))
  (bind _crystal_2 (`self.Crystal`))
  (bind _playersettings_4 (`self.PlayerSettings`))
  ;[1 1 1] Checks if Actor that overlapped box is the Player Actor
  (`|ExecutionSequence`
    (:`then_0`
      (bind _asthird_person_character (cast `/Game/GuidingLight/Core/Character/Crystal/ThirdPersonCharacter` OtherActor)))
    (:`then_1`
      (bind _asthird_person_character_2 (cast `/Game/GuidingLight/Core/Character/Crystal/ThirdPersonCharacter` (`Controller.K2_GetPawn` (`GameplayStatics.GetPlayerController` 0))))
      (bind _output_get (set `self.Crystal` _asthird_person_character_2))))
  (if (== _asthird_person_character _output_get)
    (bind _returnvalue (`GameplayStatics.DoesSaveGameExist` "CheckPoint"))
    (if _returnvalue
      ;[1 1 1] If this CheckPoint is not equal to the Current CheckPoint in the save file
      (bind _returnvalue_2 (`GameplayStatics.LoadGameFromSlot` "CheckPoint" :!label _label))
      (bind _asbp_player_settings_save (cast `/Game/GuidingLight/Settings/BP_PlayerSettingsSave` _returnvalue_2))
      (bind _output_get_2 (set `self.PlayerSettings` _asbp_player_settings_save))
      (if (not (== self (`/Game/GuidingLight/Settings/BP_PlayerSettingsSave.CurrentCheckPoint` (`self.PlayerSettings`))))
        ;[1 1 1] Update Save Game Slot and Sets New Location of Respawn
        (bind _output_get_3 (set `/Game/GuidingLight/Settings/BP_PlayerSettingsSave.Location` (`self.K2_GetActorLocation`) _output_get_2))
        (`GameplayStatics.SpawnEmitterAtLocation` "/Game/GuidingLight/Effects/Environment/P_CheckPoint.P_CheckPoint" _output_get_3 (struct) (2.0 2.0 2.0))
        (bind _output_get_4 (set `/Game/GuidingLight/Settings/BP_PlayerSettingsSave.CurrentCheckPoint` self _playersettings_4))
        (`BlueprintSetLibrary.Set_Add` (`/Game/GuidingLight/Settings/BP_PlayerSettingsSave.CheckPointPairs` _playersettings_4) _output_get_4)
        (set `/Game/GuidingLight/Settings/BP_PlayerSettingsSave.RedOrbOnPlayer` (`GuidingLightCharacter.bRedOrbInInventory` _crystal) _playersettings_2)
        (set `/Game/GuidingLight/Settings/BP_PlayerSettingsSave.BlueOrbOnPlayer` (`GuidingLightCharacter.bBlueOrbInInventory` _crystal) _playersettings_2)
        (set `/Game/GuidingLight/Settings/BP_PlayerSettingsSave.YellowOrbOnPlayer` (`GuidingLightCharacter.bYellowOrbInInventory` _crystal) _playersettings_2)
        (`GameplayStatics.SaveGameToSlot` (`self.PlayerSettings`) "CheckPoint"))
      (else
        ;[1 1 1] Create and Save Game to Slot - Sets location of Respawn
        (bind _returnvalue_3 (`GameplayStatics.CreateSaveGameObject` "/Game/GuidingLight/Settings/BP_PlayerSettingsSave.BP_PlayerSettingsSave_C"))
        (bind _output_get_5 (set `self.PlayerSettings` _returnvalue_3))
        (bind _output_get_6 (set `/Game/GuidingLight/Settings/BP_PlayerSettingsSave.Location` (`self.K2_GetActorLocation`) _output_get_5))
        (`|ExecutionSequence`
          (:`then_0`
            (`GameplayStatics.SpawnEmitterAtLocation` "/Game/GuidingLight/Effects/Environment/P_CheckPoint.P_CheckPoint" _output_get_6 (struct) (2.0 2.0 2.0))
            (bind _output_get_7 (set `/Game/GuidingLight/Settings/BP_PlayerSettingsSave.CurrentCheckPoint` self _playersettings))
            (`BlueprintSetLibrary.Set_Add` (`/Game/GuidingLight/Settings/BP_PlayerSettingsSave.CheckPointPairs` _playersettings) _output_get_7)
            (`KismetSystemLibrary.PrintString` "CheckPoint Reached!")
            (set `/Game/GuidingLight/Settings/BP_PlayerSettingsSave.RedOrbOnPlayer` (`GuidingLightCharacter.bRedOrbInInventory` _crystal_2) _playersettings_3)
            (set `/Game/GuidingLight/Settings/BP_PlayerSettingsSave.BlueOrbOnPlayer` (`GuidingLightCharacter.bBlueOrbInInventory` _crystal_2) _playersettings_3)
            (set `/Game/GuidingLight/Settings/BP_PlayerSettingsSave.YellowOrbOnPlayer` (`GuidingLightCharacter.bYellowOrbInInventory` _crystal_2) _playersettings_3)
            (`GameplayStatics.SaveGameToSlot` (`self.PlayerSettings`) "CheckPoint"))
          (:`then_1`
            (`PlayerController.PlayDynamicForceFeedback` (`GameplayStatics.GetPlayerController` 0) 2.0 1.0 true true true true)))))))

(event `self.CheckPoint2.OnComponentBeginOverlap`
  (params (OverlappedComponent :type "PrimitiveComponent Object Reference") (OtherActor :type "Actor Object Reference") (OtherComp :type "PrimitiveComponent Object Reference") (OtherBodyIndex :type Integer) (bFromSweep :type Boolean) (SweepResult :type "HitResult Structure (by ref)"))
  ;[1 1 1] Checks if Actor that overlapped box is the Player Actor
  (`|ExecutionSequence`
    (:`then_0`
      (bind _asthird_person_character (cast `/Game/GuidingLight/Core/Character/Crystal/ThirdPersonCharacter` OtherActor)))
    (:`then_1`
      (cast `/Game/GuidingLight/Core/Character/Crystal/ThirdPersonCharacter` (`Controller.K2_GetPawn` (`GameplayStatics.GetPlayerController` 0)))
      (bind _output_get (set `self.Crystal` null))))
  (if (== _asthird_person_character _output_get)
    (goto _label)))

(fn `UserConstructionScript`
  (bind _checkpoint1 (`self.CheckPoint1`))
  (bind _checkpoint2 (`self.CheckPoint2`))
  (`SceneComponent.SetHiddenInGame` _checkpoint1 (`SceneComponent.bHiddenInGame` _checkpoint1) true)
  (`SceneComponent.SetHiddenInGame` _checkpoint2 (`SceneComponent.bHiddenInGame` _checkpoint2) true))
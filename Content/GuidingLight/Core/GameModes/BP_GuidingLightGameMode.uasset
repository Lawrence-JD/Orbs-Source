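; Game mode for Guiding Light that respawns the player's ThirdPersonCharacter (Crystal) whenever it is destroyed.
; BeginPlay binds to the pawn's OnDestroyed event, and each replacement is spawned, possessed and rebound.
; Respawn location comes from the "CheckPoint" save slot, falling back to the "TheStart" player start when no save exists, with debug prints.
; The Respawn event is empty, and a health-based death animation branch is disconnected.
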(event `self.ReceiveTick`
  (params (DeltaSeconds :type "Float (single-precision)")))

(event `Respawn`
  ;[1 1 1] Binds an OnDestroyed Event on Character
)

(event `self.ReceiveBeginPlay`
  ;[1 1 1] Binds an OnDestroyed Event on Character
  (bind _asthird_person_character (cast `/Game/GuidingLight/Core/Character/Crystal/ThirdPersonCharacter` (`Controller.K2_GetPawn` (`GameplayStatics.GetPlayerController` 0))))
  (bind _output_get (set `self.Crystal` _asthird_person_character))
  (add `self.OnDestroyed` _output_get (delegate `OnDestroyed_Event`)))

(event `OnDestroyed_Event` :!signature `self.OnDestroyed`
  (params (DestroyedActor :type "Actor Object Reference"))
  (bind _returnvalue (`GameplayStatics.GetPlayerController` 0))
  (bind _returnvalue_2 (`self.K2_GetActorLocation` (`self.K2_FindPlayerStart` (`GameplayStatics.GetPlayerController` 0) "TheStart")))
  (bind _returnvalue_3 (`GameplayStatics.DoesSaveGameExist` "CheckPoint"))
  (`KismetSystemLibrary.PrintString` "Respawning" true true (struct :`R` 0.880209 :`B` 0.609115 :`A` 1.0) 30.0)
  (if _returnvalue_3
    ;[1 1 1] Spawn at Last CheckPoint/ Current Room if Check Point is setup correctly
    (bind _returnvalue_4 (`GameplayStatics.LoadGameFromSlot` "CheckPoint"))
    (bind _asbp_player_settings_save (cast `/Game/GuidingLight/Settings/BP_PlayerSettingsSave` _returnvalue_4))
    (bind _output_get (set `self.GameSettings` _asbp_player_settings_save))
    (bind _location (`/Game/GuidingLight/Settings/BP_PlayerSettingsSave.Location` _output_get))
    (bind _output_get_2 (set `self.SpawnTransform` (`KismetMathLibrary.MakeTransform` _location)))
    (`KismetSystemLibrary.PrintString` (`KismetStringLibrary.Conv_VectorToString` _location) true true (struct :`R` 1.0 :`G` 0.866591 :`A` 1.0) 15.0)
    (bind _returnvalue_5 (`|SpawnActorFromClass` "/Game/GuidingLight/Core/Character/Crystal/ThirdPersonCharacter.ThirdPersonCharacter_C" _output_get_2 "Undefined" "OverrideRootScale" null null))
    (bind _output_get_3 (set `self.Crystal` _returnvalue_5))
    (`Controller.Possess` _returnvalue _output_get_3)
    (add `self.OnDestroyed` _output_get_3 (delegate `OnDestroyed_Event`))
    (else
      ;[1 1 1] Spawn at Game Start Location if noSave Game Exists
      (bind _output_get_4 (set `self.SpawnTransform` (`KismetMathLibrary.MakeTransform` _returnvalue_2)))
      (`KismetSystemLibrary.PrintString` (`KismetStringLibrary.Conv_VectorToString` _returnvalue_2) true true (struct :`R` 1.0 :`G` 0.866591 :`A` 1.0))
      (bind _returnvalue_6 (`|SpawnActorFromClass` "/Game/GuidingLight/Core/Character/Crystal/ThirdPersonCharacter.ThirdPersonCharacter_C" _output_get_4 "Undefined" "OverrideRootScale" null null))
      (bind _output_get_5 (set `self.Crystal` _returnvalue_6))
      (`Controller.Possess` _returnvalue _output_get_5)
      (add `self.OnDestroyed` _output_get_5 (delegate `OnDestroyed_Event`))))
  (`self.Respawn`))

(fn `UserConstructionScript`)
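; Spline-based moving platform system that runs while its linked Generator's charge reaches a threshold.
; The construction script spawns NumPlatforms floating platform meshes, evenly spaced along the spline.
; The MovePlatform timeline, rate derived from Time, slides them along the spline, wrapping offsets past the end to form a conveyor.
; It restarts on finish, with Reverse adding a backward pass; below threshold it stops, or rewinds if Reverse is set.
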(event `self.ReceiveBeginPlay`
  (`TimelineComponent.SetPlayRate` (`self.MovePlatform`) (- 1.0 (/ 5.0 (`self.Time`)))))

(event `self.ReceiveTick`
  (params (DeltaSeconds :type "Float (single-precision)"))
  (bind _returnvalue (`SplineComponent.GetSplineLength` (`self.Spline`)))
  (if (> (`Generator_YellowOrb.AmountOfCharge` (`self.Generator`)) (`self.Threshold`))
    (set `self.num` (`self.Threshold`))
    (else
      (set `self.num` (`Generator_YellowOrb.AmountOfCharge` (`self.Generator`)))))
  (if (>= (`self.num`) (`self.Threshold`))
    (bind (_direction _traveldistance) (`Timeline|MovePlatform` :!label _label)
      (:`Update`
        (for (_array_element _array_index) (`self.Platforms`)
          (bind _returnvalue_2 (+ (* _traveldistance (`SplineComponent.GetSplineLength` (`self.Spline`))) (* (+ _array_index 1) (/ (`SplineComponent.GetSplineLength` (`self.Spline`)) (`KismetMathLibrary.Conv_IntToDouble` (`self.Num Platforms`))))))
          (if (> _returnvalue_2 _returnvalue)
            (`SceneComponent.K2_SetWorldLocation` _array_element (`SplineComponent.GetLocationAtDistanceAlongSpline` (`self.Spline`) (- _returnvalue_2 _returnvalue) "World") false false)
            (else
              (`SceneComponent.K2_SetWorldLocation` _array_element (`SplineComponent.GetLocationAtDistanceAlongSpline` (`self.Spline`) _returnvalue_2 "World") false false)))))
      (:`Finished`
        (if (`self.Reverse`)
          (`self.Rev`)
          (`KismetSystemLibrary.Delay` (`self.Time`))
          (goto _label :!via `PlayFromStart`)
          (else
            (goto _label :!via `PlayFromStart`)))))
    (elif (`self.Reverse`)
      (goto _label :!via `Reverse`)
      (else
        (goto _label :!via `Stop`)))))

(event `Rev`
  (goto _label :!via `Reverse`))

(fn `GetMesh`
  (returns (`Mesh Comp` :type "MeshComponent Object Reference"))
  (return null))

(fn `UserConstructionScript`
  (`KismetArrayLibrary.Array_Clear` (`self.Platforms`))
  (for _index (range 1 (+ (`self.Num Platforms`) 1))
    (bind _returnvalue (`AddComponent|NODE_AddStaticMeshComponent-0` :`RelativeTransform` (`KismetMathLibrary.Conv_VectorToTransform` (`SplineComponent.GetLocationAtDistanceAlongSpline` (`self.Spline`) (* _index (/ (`SplineComponent.GetSplineLength` (`self.Spline`)) (`KismetMathLibrary.Conv_IntToDouble` (`self.Num Platforms`)))) "Local"))))
    (`StaticMeshComponent.SetStaticMesh` _returnvalue "/Game/GuidingLight/Environment/Props/Assets/SM_P_Platform_Floating.SM_P_Platform_Floating")
    (`KismetArrayLibrary.Array_Add` (`self.Platforms`) _returnvalue)))
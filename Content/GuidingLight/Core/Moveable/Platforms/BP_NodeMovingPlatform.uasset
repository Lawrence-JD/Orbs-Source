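; BP_NodeMovingPlatform is a platform that travels through a list of node actors in a continuous loop while activated.
; Each Tick it steps its root toward the current node along a normalized direction scaled by speed, without sweeping or delta-time scaling, so speed depends on frame rate.
; Within 100 units of a node it advances the index, wrapping to the first node after the last.
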(event `self.ReceiveTick`
  (params (DeltaSeconds :type "Float (single-precision)"))
  (bind _returnvalue (- (`SceneComponent.K2_GetComponentLocation` (`/Game/GuidingLight/Core/Moveable/Platforms/BP_PlatformNode.DefaultSceneRoot` (`|GetArrayItem` (`self.BP_NodeList`) (`self.iIndex`)))) (`SceneComponent.K2_GetComponentLocation` (`self.DefaultSceneRoot`))))
  (if (and (> (`KismetArrayLibrary.Array_Length` (`self.BP_NodeList`)) 0) (`self.bActivated`))
    (if (<= (`self.iIndex`) (`KismetArrayLibrary.Array_Length` (`self.BP_NodeList`)))
      ;[1 1 1] Advances Idx if within a certain degree of completion
      (if (>= (`KismetMathLibrary.VSize` _returnvalue) 100.0) :!label _label
        (`SceneComponent.K2_SetWorldLocation` (`self.DefaultSceneRoot`) (+ (* (`KismetMathLibrary.Normal` _returnvalue) (`self.fSpeed`)) (`SceneComponent.K2_GetComponentLocation` (`self.DefaultSceneRoot`))) false false)
        (else
          (bind _result (`/Engine/EditorBlueprintResources/StandardMacros.IncrementInt` (`self.iIndex`))
            (:`  `
              (if (>= _result (`KismetArrayLibrary.Array_Length` (`self.BP_NodeList`)))
                (bind _output_get (set `self.iIndex` (- (`KismetArrayLibrary.Array_Length` (`self.BP_NodeList`)) 1)))
                (if (<= _output_get (`KismetArrayLibrary.Array_Length` (`self.BP_NodeList`)))
                  (set `self.iIndex` 0)
                  (goto _label)))))))
      (else
        (set `self.iIndex` 0)))))

(fn `UserConstructionScript`)
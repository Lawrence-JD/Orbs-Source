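; BP_Rotator_Spotlight is a moveable spotlight actor that sweeps its aim through a looping list of node actors.
; A Start/stop event toggles the motion, and while active, Tick eases rotation with RInterpTo so local -Z points at the current node.
; When the rotation is nearly aligned, it advances to the next node, wrapping to the first.
; The CollisionDetector overlap only prints a test message.
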(event `Start/stop`
  (if (`self.Go`)
    (set `self.Go` false)
    (else
      (set `self.Go` true))))

(event `self.ReceiveTick`
  (params (DeltaSeconds :type "Float (single-precision)"))
  (if (`self.Go`)
    (bind _output_get (set `self.rTargetRotation` (`KismetMathLibrary.MakeRotFromZ` (`KismetMathLibrary.Normal` (- (`self.K2_GetActorLocation`) (`self.K2_GetActorLocation` (`|GetArrayItem` (`self.bpNodeList`) (`self.iNodeIndex`))))))))
    (bind _returnvalue (`KismetMathLibrary.RInterpTo` (`self.K2_GetActorRotation`) _output_get DeltaSeconds 0.5))
    (`self.K2_SetActorRotation` _returnvalue)
    (if (== _returnvalue (`self.rTargetRotation`) :`ErrorTolerance` 1.0)
      (`/Engine/EditorBlueprintResources/StandardMacros.IncrementInt` (`self.iNodeIndex`)
        (:`  `
          (if (>= (`self.iNodeIndex`) (`KismetArrayLibrary.Array_Length` (`self.bpNodeList`)))
            (set `self.iNodeIndex` 0)))))))

(event `self.Collision detector.OnComponentBeginOverlap`
  (params (OverlappedComponent :type "PrimitiveComponent Object Reference") (OtherActor :type "Actor Object Reference") (OtherComp :type "PrimitiveComponent Object Reference") (OtherBodyIndex :type Integer) (bFromSweep :type Boolean) (SweepResult :type "HitResult Structure (by ref)"))
  (`KismetSystemLibrary.PrintString` "Testing"))

(fn `UserConstructionScript`)
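; BP_PlatformSpline is a moving platform that travels once along a spline when StartPlatform is called, then bobs in place.
; A timeline, with its play rate set by Speed, drives position by spline distance while rotation blends toward the spline's end rotation as remaining distance shrinks.
; On finishing, Tick oscillates the platform vertically around its arrival height by BobDistance, starting randomly up or down.
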(event `self.ReceiveTick`
  (params (DeltaSeconds :type "Float (single-precision)"))
  (bind _spline (`self.Spline`))
  (bind _bobanchor (`self.BobAnchor`))
  (bind _returnvalue (`SplineComponent.GetSplineLength` (`self.Spline`)))
  (bind _z (.z (`SceneComponent.K2_GetComponentLocation` (`self.Platform`))))
  (`|ExecutionSequence`
    (:`then_0`
      (if (`self.bStart`)
        (`/Engine/EditorBlueprintResources/StandardMacros.DoOnce` false
          (:`Completed`
            (bind (_direction _alpha) (`Timeline|Timeline_0`)
              (:`Update`
                (`TimelineComponent.SetPlayRate` (`self.Timeline_0`) (`self.Speed`))
                (bind _returnvalue_2 (`KismetMathLibrary.Lerp` 0.0 _returnvalue _alpha))
                (`SceneComponent.K2_SetWorldLocation` (`self.Platform`) (`SplineComponent.GetLocationAtDistanceAlongSpline` (`self.Spline`) _returnvalue_2 "World") false false)
                (`SceneComponent.K2_SetWorldRotation` (`self.Platform`) (`KismetMathLibrary.RLerp` (`SceneComponent.K2_GetComponentRotation` (`self.Platform`)) (`SplineComponent.GetRotationAtSplinePoint` _spline (`SplineComponent.GetNumberOfSplinePoints` _spline) "World") (/ (`KismetMathLibrary.Conv_IntToDouble` (`SplineComponent.GetNumberOfSplinePoints` (`self.Spline`))) (- _returnvalue _returnvalue_2))) false false))
              (:`Finished`
                (set `self.bBob` true)
                (set `self.BobAnchor` (.z (`SceneComponent.K2_GetComponentLocation` (`self.Platform`))))
                (if (`KismetMathLibrary.RandomBool`)
                  (set `self.BobToggler` 1.0)
                  (else
                    (set `self.BobToggler` -1.0)))))))))
    (:`then_1`
      (if (`self.bBob`)
        (`SceneComponent.K2_SetWorldLocation` (`self.Platform`) (`KismetMathLibrary.MakeVector` (.x (`SceneComponent.K2_GetComponentLocation` (`self.Platform`))) (.y (`SceneComponent.K2_GetComponentLocation` (`self.Platform`))) (+ (.z (`SceneComponent.K2_GetComponentLocation` (`self.Platform`))) (* (* (`self.BobDistance`) DeltaSeconds) (`self.BobToggler`)))) false false)
        (if (or (>= _z (+ _bobanchor (`self.BobDistance`))) (<= _z (- _bobanchor (`self.BobDistance`))))
          (set `self.BobToggler` (* (`self.BobToggler`) -1.0)))))))

(fn `StartPlatform`
  (set `self.bStart` true))

(fn `UserConstructionScript`)
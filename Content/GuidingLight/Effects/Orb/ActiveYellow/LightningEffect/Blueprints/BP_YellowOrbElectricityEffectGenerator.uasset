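; Electricity generator for the yellow orb effect that, while active, repeatedly spawns BP_SpawnedArc lightning at random short intervals.
; Arcs either strike spherically at random or run point to point toward a target, switched by SetToDirected and SetToUndirected.
; Location Logic derives point-to-point endpoints from vectors or actors, and Setup Arc Struct packs the arc settings.
; A self-looping timer flickers the core material and light, continuing after deactivation hides the components.
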(event `Arcing`
  (bind _returnvalue (`self.K2_GetActorLocation`))
  (bind _destination_object (`self.Destination Object`))
  (bind _branch_count (`self.Branch Count`))
  (bind (_distance _boltcolor _isbranch _allowbranches _branchlimit _priorhitloc _priorhitnormal _playrate _customvectors _origin _dest _noisescale _noisespeed) (break `/Game/GuidingLight/Effects/Orb/ActiveYellow/LightningEffect/Blueprints/ArcValues` (`self.Arc Struct`)))
  (bind _returnvalue_2 (- (`self.K2_GetActorLocation` _destination_object) _returnvalue))
  ;[1 1 1] Create arc
  (bind _returnvalue_3 (`|SpawnActorFromClass` "/Game/GuidingLight/Effects/Orb/ActiveYellow/LightningEffect/Blueprints/BP_SpawnedArc.BP_SpawnedArc_C" (`self.GetTransform`) "Undefined" "OverrideRootScale" self (`self.Movable`) null))
  (bind _output_get (set `self.Arc Struct` (make `/Game/GuidingLight/Effects/Orb/ActiveYellow/LightningEffect/Blueprints/ArcValues` (`self.Arc Radius`) (`self.ArcColor`) false (>= _branch_count 1) _branch_count (0.0 0.0 0.0) (0.0 0.0 0.0) 0.0 false (`self.Passalong_O`) (`self.Passalong_D`) (`self.Arc Noise Scale`) (`self.Arc Noise Speed`))))
  (switch `/Game/GuidingLight/Effects/Orb/ActiveYellow/LightningEffect/Blueprints/ArcStyle` (`self.Style Selector`)
    (:`NewEnumerator0`
      ;[1 0.3698 0.3698] Pass spawning values to arc
      (`/Game/GuidingLight/Effects/Orb/ActiveYellow/LightningEffect/Blueprints/BP_SpawnedArc.Spawn` _returnvalue_3 _output_get)
      ;[0.6678 1 0.7297] Spawn new arc
      (`KismetSystemLibrary.Delay` (`KismetMathLibrary.RandomFloatInRange` (`self.Arc Min Delay`) (`self.Arc Max Delay`)) :!label _label)
      (if (`self.bIsActive`)
        (`self.Arcing`)))
    (:`NewEnumerator1`
      ;[1 0.3698 0.3698] Pass spawning values to arc
      (switch `/Game/GuidingLight/Effects/Orb/ActiveYellow/LightningEffect/Blueprints/Endpoints` (`self.Point Selector`)
        (:`NewEnumerator0`
          (`|ExecutionSequence`
            (:`then_0`
              (set `self.Passalong_O` (`KismetMathLibrary.Vector_Zero`) :!label _label_2))
            (:`then_1`
              (set `self.Passalong_D` (`self.Destination`)))
            (:`then_2`
              (`/Game/GuidingLight/Effects/Orb/ActiveYellow/LightningEffect/Blueprints/BP_SpawnedArc.Spawn` _returnvalue_3 (make `/Game/GuidingLight/Effects/Orb/ActiveYellow/LightningEffect/Blueprints/ArcValues` _distance _boltcolor _isbranch _allowbranches _branchlimit _priorhitloc _priorhitnormal _playrate true _origin _dest _noisescale _noisespeed) :!label _label_3)
              (goto _label))))
        (:`NewEnumerator1`
          (bind _asstatic_mesh_actor (cast `StaticMeshActor` _destination_object))
          (`KismetSystemLibrary.PrintString` "Got Mesh"))
        (:`NewEnumerator2`
          (`|ExecutionSequence`
            (:`then_0`
              (goto _label_2))
            (:`then_1`
              (bind _output_get_2 (set `self.Passalong_D` _returnvalue_2))
              (set `self.Passalong_D` (`KismetMathLibrary.RotateAngleAxis` _output_get_2 (* (`KismetMathLibrary.DegAtan2` (- (.x (`KismetMathLibrary.Vector_Forward`)) (.x (`KismetMathLibrary.GetForwardVector` (`self.K2_GetActorRotation`)))) (- (.y (`KismetMathLibrary.Vector_Forward`)) (.y (`KismetMathLibrary.GetForwardVector` (`self.K2_GetActorRotation`))))) 2.0) (`self.GetActorUpVector`))))
            (:`then_2`
              (goto _label_3))))
        (:`NewEnumerator3`
          (`|ExecutionSequence`
            (:`then_0`
              (set `self.Passalong_O` (- (`self.K2_GetActorLocation` (`self.Origin Object`)) _returnvalue)))
            (:`then_1`
              (set `self.Passalong_D` _returnvalue_2))
            (:`then_2`
              (goto _label_3))))))))

(event `Set To Directed`
  (params (TargetActor :type "Actor Object Reference"))
  ;[1 1 1] Set Generator To Be Directed At A Target
  (set `self.Style Selector` "NewEnumerator1")
  (set `self.Origin` (`self.K2_GetActorLocation`))
  (set `self.Destination` (`self.K2_GetActorLocation` TargetActor))
  (set `self.ArcColor` (struct :`R` 0.924709 :`G` 0.93 :`B` 0.765313 :`A` 76.404541))
  (set `self.Origin Object` self)
  (set `self.Destination Object` TargetActor))

(event `Set To Undirected`
  ;[1 1 1] Set Generator To Fire At Random Surfaces
  (set `self.Style Selector` "NewEnumerator0")
  (set `self.ArcColor` (struct :`R` 0.93 :`G` 0.823842 :`B` 0.164442 :`A` 76.404541)))

(event `Set Target Location`
  (params (TargetLocation :type "Vector Structure"))
  ;[1 1 1] Set Destination For Lightning Generator
  (set `self.Destination` TargetLocation))

(event `ActivateGenerator`
  ;[1 1 1] Activates Generator
  (set `self.bIsActive` true)
  (`SceneComponent.SetHiddenInGame` (`self.DefaultSceneRoot`) false true)
  ;[0.3491 0.5682 1] Initialization
  (`KismetSystemLibrary.K2_SetTimer` null "RandomCoreSize" 0.05)
  (`KismetSystemLibrary.K2_SetTimer` null "Arcing" (`KismetMathLibrary.RandomFloatInRange` 0.05 0.025)))

(event `DeactivateGenerator`
  ;[1 1 1] Deactivate Generator
  (set `self.bIsActive` false)
  (`SceneComponent.SetHiddenInGame` (`self.DefaultSceneRoot`) true true))

(event `RandomCoreSize`
  ;[1 0.9123 0.5649] Light setup for core (flickers size and brightness)
  (`MaterialInstanceDynamic.SetVectorParameterValue` (`self.SphereMat`) "Color" (* (`self.ArcColor`) (`KismetMathLibrary.RandomFloatInRange` 1.0 5.0)))
  (`LightComponent.SetIntensity` (`self.PointLight`) (`KismetMathLibrary.RandomFloatInRange` 320.0 5000.0))
  (`KismetSystemLibrary.Delay` (`KismetMathLibrary.RandomFloatInRange` 0.05 0.09))
  (`self.RandomCoreSize`))

(fn `UserConstructionScript`
  (`SphereComponent.SetSphereRadius` (`self.Radius Indicator`) (`self.Arc Radius`) true) ; Show the area the arcs will strike
  ;[1 1 1] Pass color to components
  (`LightComponent.SetLightColor` (`self.PointLight`) (`self.ArcColor`) true)
  (bind _returnvalue (`PrimitiveComponent.CreateDynamicMaterialInstance` (`self.Shape_Sphere`) 0 null "None"))
  (bind _output_get (set `self.SphereMat` _returnvalue))
  (`MaterialInstanceDynamic.SetVectorParameterValue` _output_get "Color" (`self.ArcColor`))
  (`SceneComponent.SetHiddenInGame` (`self.Shape_Sphere`) (not (`self.bCoreVisible`)) false))